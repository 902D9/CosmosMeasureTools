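; Controller for the Cosmos measure tools that drives an in-game distance measuring tool with the mouse.
; On BeginPlay it spawns a BP_CosmosDistanceMeasureTool and immediately starts a non-complex measurement.
; Left click adds a point while measuring, or restarts measuring with a shorter distance setting than the initial one.
; Right click stops the measurement.
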(event `self.ReceiveBeginPlay`
  (bind _returnvalue (`|SpawnActorFromClass` "/CosmosMeasureTools/BP_CosmosDistanceMeasureTool.BP_CosmosDistanceMeasureTool_C" (`KismetMathLibrary.MakeTransform` (0.0 0.0 0.0)) "AlwaysSpawn" "OverrideRootScale" null null))
  (bind _output_get (set `self.CosmosDistanceMeasureTool` _returnvalue))
  (`CosmosMeasureTool.StartMeasuring` _output_get false 100000.0))

(event `Key|LeftMouseButton`
  (params (Key :type "Key Structure"))
  (bind _cosmosdistancemeasuretool (`self.CosmosDistanceMeasureTool`))
  (:`Pressed`
    (if (`CosmosMeasureTool.bMeasuring` _cosmosdistancemeasuretool)
      (`CosmosMeasureTool.AddMeasuringPoint` _cosmosdistancemeasuretool)
      (else
        (`CosmosMeasureTool.StartMeasuring` _cosmosdistancemeasuretool false 10000.0)))))

(event `Key|RightMouseButton`
  (params (Key :type "Key Structure"))
  (:`Pressed`
    (`CosmosMeasureTool.StopMeasuring` (`self.CosmosDistanceMeasureTool`))))

(fn `UserConstructionScript`)